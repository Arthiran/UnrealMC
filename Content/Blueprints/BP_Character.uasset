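; Player character for a Minecraft-style voxel game that breaks and places blocks, with hotkeys selecting the block type.
; BeginPlay creates the UI and locks input and movement until a timer sees BP_ChunkWorld's IsStarted clear.
; Mouse clicks trace from the camera, offset by hit normal to edit chunk voxels, and play material-specific sounds.
; Tick toggles underwater post-process and sounds via a height-gated Water trace, and teleports fallen players back up.
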(event Custom|WaitForChunk
  (if (not (Variables|/Script/UnrealMC.ChunkWorld|GetbIsStarted (Variables|Default|GetBP_ChunkWorld)))
    (Input|EnableInput (Game|Player|GetPlayerPawn 0) (Game|GetPlayerController 0))
    (Pawn|Components|CharacterMovement|SetMovementMode (Variables|Character|GetCharacterMovement) "MOVE_Walking" 0)
    (Utilities|Time|ClearandInvalidateTimerbyHandle (Variables|Default|GetChunkHandle))
    (Utilities|FlowControl|Delay 3.0)
    (Widget|SetVisibility (Variables|/Game/Blueprints/Widgets/WBP_UI.WBP_UI_C|GetWBP_MinecraftBG (Variables|Default|GetUI)) "Hidden")))

(event EventBeginPlay
  (Input|DisableInput (Game|GetPlayerController 0))
  (Pawn|Components|CharacterMovement|DisableMovement (Variables|Character|GetCharacterMovement))
  (bind _outactors (Actor|GetAllActorsOfClass "/Game/Blueprints/BP_ChunkWorld.BP_ChunkWorld_C"))
  (if (== (Utilities|Array|Length _outactors) 1)
    (bind _output_get (Variables|Default|SetBP_ChunkWorld (Utilities|Array|Get(acopy) _outactors)))
    (Variables|Default|SetChunkSize (Variables|/Script/UnrealMC.ChunkWorld|GetSize _output_get))
    (bind _returnvalue (UserInterface|CreateWidget "/Game/Blueprints/Widgets/WBP_UI.WBP_UI_C" (Game|GetPlayerController 0)))
    (bind _output_get_2 (Variables|Default|SetUI _returnvalue))
    (UserInterface|Viewport|AddtoViewport _output_get_2 0)
    (bind _returnvalue_2 (Utilities|Time|SetTimerbyEvent (delegate Custom|WaitForChunk) 1.0 true))
    (Variables|Default|SetChunkHandle _returnvalue_2)))

(event EventTick
  (params (DeltaSeconds :type Float%20%28single-precision%29))
  (bind _returnvalue (Transformation|GetActorLocation))
  (bind _returnvalue_2 (Transformation|GetActorLocation))
  (if (and (< (.z _returnvalue) 3.38e+04) (> (.z _returnvalue) 3.12e+04))
    (bind (_outhit _returnvalue_3) (Collision|LineTraceByChannel _returnvalue_2 (* _returnvalue_2 (* (Transformation|GetActorUpVector) 2e+03)) "TraceTypeQuery3" false 0 "None" true "(R=1.000000,G=0.000000,B=0.000000,A=1.000000)" "(R=0.000000,G=1.000000,B=0.000000,A=1.000000)" 3.0))
    (if _returnvalue_3
      (if (.bSuccess (Utilities|Casting|CastToWater (.HitActor (Collision|BreakHitResult _outhit))))
        (if (not (Variables|Default|GetAlreadyOn))
          (CallFunction|SwitchPP true)
          (Variables|Default|SetAlreadyOn true)
          (Variables|Default|SetAlreadyOff false)
          (Audio|PlaySoundatLocation "/Game/Sounds/Water/SC_Water_Enter.SC_Water_Enter" (Transformation|GetActorLocation) "0, 0, 0" 1.0 1.0 0.0 0 0 0 0))
        (else
          (if (not (Variables|Default|GetAlreadyOff)) :!label _label
            (CallFunction|SwitchPP false)
            (Variables|Default|SetAlreadyOn false)
            (Variables|Default|SetAlreadyOff true)
            (Audio|PlaySoundatLocation "/Game/Sounds/Water/SC_Water_Exit.SC_Water_Exit" (Transformation|GetActorLocation) "0, 0, 0" 1.0 1.0 0.0 0 0 0 0))))
      (else
        (goto _label)))
    (elif (< (.z _returnvalue) -3e+02)
      (Transformation|SetActorLocation (Math|Vector|MakeVector (+ (.x _returnvalue) 1e+02) (+ (.y _returnvalue) 1e+02) 4e+04) false false)
      (goto _label)
      (else
        (goto _label)))))

(event Input|KeyboardEvents|Escape
  (params (Key :type Key%20Structure :default "None"))
  (:Pressed
    (Default|OpenPauseScreen (Variables|Default|GetUI) (Game|GetPlayerController 0))))

(event Input|MouseEvents|RightMouseButton
  (params (Key :type Key%20Structure :default "None"))
  (bind _bp_chunkworld (Variables|Default|GetBP_ChunkWorld))
  (bind _chunksize (Variables|Default|GetChunkSize))
  (:Pressed
    (bind (_outhit _returnvalue) (CallFunction|BlockCast))
    (if _returnvalue
      (Utilities|Casting|CastToChunkBase (.HitActor (Collision|BreakHitResult _outhit)))
      (Utilities|IsValid _bp_chunkworld
        (:Is%20Valid
          (if (not (Class|KismetMathLibrary|EqualExactlyVectorVector (Math|Conversions|ToVector(Float) (Class|VoxelFunctionLibrary|WorldtoLocalBlockPosition (+ (.Location (Collision|BreakHitResult _outhit)) (* (.Normal (Collision|BreakHitResult _outhit)) 50)) _chunksize)) (Math|Conversions|ToVector(Float) (Class|VoxelFunctionLibrary|WorldtoLocalBlockPosition (Transformation|GetActorLocation (Game|Player|GetPlayerPawn 0)) _chunksize))))
            (bind _returnvalue_2 (Class|ChunkWorld|FindandModifyChunk _bp_chunkworld (Class|KismetMathLibrary|FTruncVector (+ (.Location (Collision|BreakHitResult _outhit)) (* (.Normal (Collision|BreakHitResult _outhit)) 50))) (Class|VoxelFunctionLibrary|WorldtoLocalBlockPosition (+ (.Location (Collision|BreakHitResult _outhit)) (* (.Normal (Collision|BreakHitResult _outhit)) 50)) _chunksize) (Variables|Default|GetBlockToPlace)))
            (bind _asbp_character (Utilities|Casting|CastToBP_Character (Game|Player|GetPlayerPawn 0)))
            (switch Utilities|FlowControl|Switch|SwitchonEBlock _returnvalue_2
              (:Stone
                (Audio|PlaySoundatLocation "/Game/Sounds/Digging/SC_Digging_Stone.SC_Digging_Stone" (Transformation|GetActorLocation _asbp_character) "0, 0, 0" 1.0 1.0 0.0 0 0 _asbp_character 0))
              (:Dirt
                (Audio|PlaySoundatLocation "/Game/Sounds/Digging/SC_Digging_Gravel.SC_Digging_Gravel" (Transformation|GetActorLocation _asbp_character) "0, 0, 0" 1.0 1.0 0.0 0 0 _asbp_character 0 :!label _label))
              (:Grass
                (goto _label))
              (:Oak
                (Audio|PlaySoundatLocation "/Game/Sounds/Digging/SC_Digging_Wood.SC_Digging_Wood" (Transformation|GetActorLocation _asbp_character) "0, 0, 0" 1.0 1.0 0.0 0 0 _asbp_character 0 :!label _label_2))
              (:OakLeaves
                (goto _label_2)))))))))

(event Input|KeyboardEvents|7
  (params (Key :type Key%20Structure :default "None"))
  (:Pressed
    (Variables|Default|SetBlockToPlace "Black_Concrete")))

(event Input|KeyboardEvents|8
  (params (Key :type Key%20Structure :default "None"))
  (:Pressed
    (Variables|Default|SetBlockToPlace "Red_Concrete")))

(event Input|KeyboardEvents|9
  (params (Key :type Key%20Structure :default "None"))
  (:Pressed
    (Variables|Default|SetBlockToPlace "White_Concrete")))

(event Input|MouseEvents|LeftMouseButton
  (params (Key :type Key%20Structure :default "None"))
  (:Pressed
    (bind (_outhit _returnvalue) (CallFunction|BlockCast))
    (if _returnvalue
      (bind _aschunk_base (Utilities|Casting|CastToChunkBase (.HitActor (Collision|BreakHitResult _outhit))))
      (bind _returnvalue_2 (Class|ChunkBase|ModifyVoxel _aschunk_base (Class|VoxelFunctionLibrary|WorldtoLocalBlockPosition (- (.Location (Collision|BreakHitResult _outhit)) (.Normal (Collision|BreakHitResult _outhit))) (Variables|Default|GetChunkSize)) "Air"))
      (bind _asbp_character (Utilities|Casting|CastToBP_Character (Game|Player|GetPlayerPawn 0)))
      (switch Utilities|FlowControl|Switch|SwitchonEBlock _returnvalue_2
        (:Stone
          (Audio|PlaySoundatLocation "/Game/Sounds/Digging/SC_Digging_Stone.SC_Digging_Stone" (Transformation|GetActorLocation _asbp_character) "0, 0, 0" 1.0 1.0 0.0 0 0 _asbp_character 0))
        (:Dirt
          (Audio|PlaySoundatLocation "/Game/Sounds/Digging/SC_Digging_Gravel.SC_Digging_Gravel" (Transformation|GetActorLocation _asbp_character) "0, 0, 0" 1.0 1.0 0.0 0 0 _asbp_character 0 :!label _label))
        (:Grass
          (goto _label))
        (:Oak
          (Audio|PlaySoundatLocation "/Game/Sounds/Digging/SC_Digging_Wood.SC_Digging_Wood" (Transformation|GetActorLocation _asbp_character) "0, 0, 0" 1.0 1.0 0.0 0 0 _asbp_character 0 :!label _label_2))
        (:OakLeaves
          (goto _label_2))))))

(event Input|KeyboardEvents|1
  (params (Key :type Key%20Structure :default "None"))
  (:Pressed
    (Default|ChangeSelectedBoxPosition (Variables|Default|GetUI))
    (Variables|Default|SetBlockToPlace "Grass")))

(event Input|KeyboardEvents|4
  (params (Key :type Key%20Structure :default "None"))
  (:Pressed
    (Default|ChangeSelectedBoxPosition (Variables|Default|GetUI) 3)
    (Variables|Default|SetBlockToPlace "Oak")))

(event Input|KeyboardEvents|5
  (params (Key :type Key%20Structure :default "None"))
  (:Pressed
    (Variables|Default|SetBlockToPlace "Brown_Concrete")))

(event Input|KeyboardEvents|2
  (params (Key :type Key%20Structure :default "None"))
  (:Pressed
    (Default|ChangeSelectedBoxPosition (Variables|Default|GetUI) 1)
    (Variables|Default|SetBlockToPlace "Dirt")))

(event Input|KeyboardEvents|3
  (params (Key :type Key%20Structure :default "None"))
  (:Pressed
    (Default|ChangeSelectedBoxPosition (Variables|Default|GetUI) 2)
    (Variables|Default|SetBlockToPlace "Stone")))

(event Input|KeyboardEvents|0
  (params (Key :type Key%20Structure :default "None"))
  (:Pressed
    (Variables|Default|SetBlockToPlace "Blue_Concrete")))

(event Input|KeyboardEvents|6
  (params (Key :type Key%20Structure :default "None"))
  (:Pressed
    (Variables|Default|SetBlockToPlace "Orange_Concrete")))

(fn ConstructionScript)

(fn SwitchPP
  (params (bOn :type Boolean))
  (if bOn
    (Variables|/Script/Engine.PostProcessComponent|SetSettings (Variables|Default|GetPostProcess) (Utilities|Struct|MakePostProcessSettings (Utilities|Struct|MakeWeightedBlendables (Utilities|Array|MakeArray (Utilities|Struct|MakeWeightedBlendable 1.0 (.Object (Utilities|Struct|BreakWeightedBlendable (Utilities|Array|Get(acopy) (.array (Utilities|Struct|BreakPostProcessSettings (Variables|/Script/Engine.PostProcessComponent|GetSettings (Variables|Default|GetPostProcess))))))))))))
    (Variables|Default|SetPPOn true)
    (else
      (Variables|/Script/Engine.PostProcessComponent|SetSettings (Variables|Default|GetPostProcess) (Utilities|Struct|MakePostProcessSettings (Utilities|Struct|MakeWeightedBlendables (Utilities|Array|MakeArray (Utilities|Struct|MakeWeightedBlendable 0.0 (.Object (Utilities|Struct|BreakWeightedBlendable (Utilities|Array|Get(acopy) (.array (Utilities|Struct|BreakPostProcessSettings (Variables|/Script/Engine.PostProcessComponent|GetSettings (Variables|Default|GetPostProcess))))))))))))
      (Variables|Default|SetPPOn false))))

(fn BlockCast
  (bind _followcamera (Variables|Default|GetFollowCamera))
  (bind _returnvalue (Transformation|GetWorldLocation _followcamera))
  (bind (_outhit _returnvalue_2) (Collision|LineTraceByChannel _returnvalue (+ _returnvalue (* (Math|Vector|GetForwardVector (Transformation|GetWorldRotation _followcamera)) (Variables|Default|GetBlockDistance))) "TraceTypeQuery4" false 0 "None" true "(R=1.000000,G=0.000000,B=0.000000,A=1.000000)" "(R=0.000000,G=1.000000,B=0.000000,A=1.000000)" 3.0))
  (return _outhit _returnvalue_2))
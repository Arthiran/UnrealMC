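; Pawn Blueprint that toggles a post-process material according to whether a line trace hits Water, likely an underwater effect.
; Each Tick within a fixed Z band, it traces from its location to that location multiplied, rather than offset, by its scaled up vector.
; SwitchPP rebuilds the PostProcess settings with the first blendable at full weight on a Water hit, zero otherwise.
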(event EventTick
  (params (DeltaSeconds :type Float%20%28single-precision%29))
  (bind _returnvalue (Transformation|GetActorLocation))
  (bind _returnvalue_2 (Transformation|GetActorLocation))
  (if (and (< (.z _returnvalue) 3.38e+04) (> (.z _returnvalue) 3.12e+04))
    (bind (_outhit _returnvalue_3) (Collision|LineTraceByChannel _returnvalue_2 (* _returnvalue_2 (* (Transformation|GetActorUpVector) 2e+03)) "TraceTypeQuery3" false 0 "None" true "(R=1.000000,G=0.000000,B=0.000000,A=1.000000)" "(R=0.000000,G=1.000000,B=0.000000,A=1.000000)" 1e+01))
    (if _returnvalue_3
      (if (.bSuccess (Utilities|Casting|CastToWater (.HitActor (Collision|BreakHitResult _outhit))))
        (CallFunction|SwitchPP true)
        (else
          (CallFunction|SwitchPP false :!label _label)))
      (else
        (goto _label)))
    (else
      (goto _label))))

(fn ConstructionScript)

(fn SwitchPP
  (params (bOn :type Boolean))
  (bind _postprocess (Variables|Default|GetPostProcess))
  (bind _postprocess_2 (Variables|Default|GetPostProcess))
  (if bOn
    (Variables|/Script/Engine.PostProcessComponent|SetSettings _postprocess_2 (Utilities|Struct|MakePostProcessSettings (Utilities|Struct|MakeWeightedBlendables (Utilities|Array|MakeArray (Utilities|Struct|MakeWeightedBlendable 1.0 (.Object (Utilities|Struct|BreakWeightedBlendable (Utilities|Array|Get(acopy) (.array (Utilities|Struct|BreakPostProcessSettings (Variables|/Script/Engine.PostProcessComponent|GetSettings _postprocess_2)))))))))))
    (else
      (Variables|/Script/Engine.PostProcessComponent|SetSettings _postprocess (Utilities|Struct|MakePostProcessSettings (Utilities|Struct|MakeWeightedBlendables (Utilities|Array|MakeArray (Utilities|Struct|MakeWeightedBlendable 0.0 (.Object (Utilities|Struct|BreakWeightedBlendable (Utilities|Array|Get(acopy) (.array (Utilities|Struct|BreakPostProcessSettings (Variables|/Script/Engine.PostProcessComponent|GetSettings _postprocess))))))))))))))
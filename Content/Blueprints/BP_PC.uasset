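; Player controller for a chunk-based block world that drives chunk updates as the player moves and applies graphics settings.
; BeginPlay sets a quality preset through scalability console commands, locks input to the game and, after a short delay, caches the single BP_ChunkWorld.
; Tick converts pawn location to chunk coordinates and calls UpdateChunks only when they change.
; BlockCast provides a camera-forward line trace; other quality presets are left unwired.
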(event EventTick
  (params (DeltaSeconds :type Float%20%28single-precision%29))
  (bind _returnvalue (Game|Player|GetPlayerPawn 0))
  (bind _bp_chunkworld (Variables|Default|GetBP_ChunkWorld))
  (bind _returnvalue_2 (Transformation|GetActorLocation _returnvalue))
  (bind _returnvalue_3 (Class|VoxelFunctionLibrary|WorldtoChunkPosition _returnvalue_2 16))
  (Utilities|IsValid _bp_chunkworld
    (:Is%20Valid
      (if (Utilities|Operators|NotEqual(!=) (Math|Conversions|ToVector(Float) (Variables|Default|GetPlayerPosition)) (Math|Conversions|ToVector(Float) _returnvalue_3) 0.0)
        (Class|ChunkWorld|UpdateChunks _bp_chunkworld _returnvalue_3)
        (Variables|Default|SetPlayerPosition _returnvalue_3)))))

(event EventBeginPlay
  (CallFunction|SetQuality "2" "50")
  (Input|SetInputModeGameOnly self)
  (Variables|Default|SetbShowMouseCursor false)
  (Utilities|FlowControl|Delay 1.0)
  (bind _outactors (Actor|GetAllActorsOfClass "/Game/Blueprints/BP_ChunkWorld.BP_ChunkWorld_C"))
  (if (== (Utilities|Array|Length _outactors) 1)
    (Variables|Default|SetBP_ChunkWorld (Utilities|Array|Get(acopy) _outactors))))

(fn ConstructionScript)

(fn BlockCast
  (bind _playercameramanager (Variables|Default|GetPlayerCameraManager))
  (bind _returnvalue (Camera|GetCameraLocation _playercameramanager))
  (bind (_outhit _returnvalue_2) (Collision|LineTraceByChannel _returnvalue (+ _returnvalue (* (Math|Vector|GetForwardVector (Camera|GetCameraRotation _playercameramanager)) (Variables|Default|GetBlockDistance))) "TraceTypeQuery4" false 0 "None" true "(R=1.000000,G=0.000000,B=0.000000,A=1.000000)" "(R=0.000000,G=1.000000,B=0.000000,A=1.000000)" 1e+01))
  (return _outhit _returnvalue_2))

(fn SetQuality
  (params (QualityValue :type String) (ResolutionValue :type String))
  (Development|ExecuteConsoleCommand (Utilities|String|Append "sg.ResolutionQuality " ResolutionValue) 0)
  (Development|ExecuteConsoleCommand (Utilities|String|Append "sg.AntiAliasingQuality " QualityValue) 0)
  (Development|ExecuteConsoleCommand (Utilities|String|Append "sg.PostProcessQuality " QualityValue) 0)
  (Development|ExecuteConsoleCommand (Utilities|String|Append "sg.ShadowQuality " QualityValue) 0)
  (Development|ExecuteConsoleCommand (Utilities|String|Append "sg.GlobalIlluminationQuality " QualityValue) 0)
  (Development|ExecuteConsoleCommand (Utilities|String|Append "sg.ReflectionQuality " QualityValue) 0)
  (Development|ExecuteConsoleCommand (Utilities|String|Append "sg.TextureQuality " QualityValue) 0)
  (Development|ExecuteConsoleCommand (Utilities|String|Append "sg.EffectsQuality " QualityValue) 0)
  (Development|ExecuteConsoleCommand (Utilities|String|Append "sg.FoliageQuality " QualityValue) 0)
  (Development|ExecuteConsoleCommand (Utilities|String|Append "sg.ShadingQuality " QualityValue) 0))